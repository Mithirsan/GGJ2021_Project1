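; Local multiplayer spawner actor that creates the players and their characters and serves as the view for player 0.
; On BeginPlay it takes the camera, creates local players, caches their BP_PlayerControllers, then spawns a BP_PlayerCharacter per player at optionally shuffled SpawnsLocations.
; Each character gets a PlayerId and is possessed by its controller, with the view target reapplied afterwards.
; The construction script sets spring arm length and adds a box component per spawn location.
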(event Custom|CreatePlayersIDs
  ;[0 1 0] Create Player controllers with IDs
  (for _index (range 0 (- (Variables|Default|GetNumberOfPlayer) 1))
    (Class|GameplayStatics|CreatePlayer _index)
    (bind _asbp_player_controller (Utilities|Casting|CastToBP_PlayerController (Game|GetPlayerController _index)))
    (Utilities|Array|Add (Variables|Default|GetPlayerController) _asbp_player_controller))
  (CallFunction|CreatePawns))

(event Custom|CreatePawns
  ;[0 1 0] CreatePlayers Charcater/Pawn
  (if (Variables|Default|GetRandomize?)
    (Utilities|Array|Shuffle (Variables|Default|GetSpawnsLocations)))
  (for _index (range 0 (- (Variables|Default|GetNumberOfPlayer) 1))
    (bind _returnvalue (Game|SpawnActorfromClass "/Game/Blueprints/BP_PlayerCharacter.BP_PlayerCharacter_C" (Math|Transform|MakeTransform (Utilities|Array|Get(acopy) (Variables|Default|GetSpawnsLocations) _index)) "AdjustIfPossibleButAlwaysSpawn" 0 0))
    (Variables|/Game/Blueprints/BP_PlayerCharacter.BP_PlayerCharacter_C|SetPlayerId _returnvalue _index)
    (Utilities|Array|Add (Variables|Default|GetCharacters) _returnvalue))
  (CallFunction|PossesCharswithPControllers))

(event Custom|PossesCharsWithPControllers
  ;[0.04841 1 0] Posses Chacters With Player Controllers
  (for _index (range 0 (- (Variables|Default|GetNumberOfPlayer) 1))
    (Pawn|Possess (Utilities|Array|Get(acopy) (Variables|Default|GetPlayerController) _index) (Utilities|Array|Get(acopy) (Variables|Default|GetCharacters) _index))
    (CallFunction|SwitchCamera)))

(event Custom|SwitchCamera
  (Game|Player|SetViewTargetwithBlend (Game|GetPlayerController 0) self 0.0 "VTBlend_Linear" 0.0 false))

(event EventBeginPlay
  ;[0 1 0] Begin Play
  (CallFunction|SwitchCamera)
  (CallFunction|CreatePlayersIDs))

(fn ConstructionScript
  (Variables|/Script/Engine.SpringArmComponent|SetTargetArmLength (Variables|Default|GetSpringArm) (Variables|Default|GetArm%20Length))
  (for _array_element (Variables|Default|GetSpawnsLocations)
    (bind _returnvalue (AddComponent|AddBoxComponent true (Math|Transform|MakeTransform (Math|Vector|MakeVector (.X (Math|Vector|BreakVector _array_element)) (.Y (Math|Vector|BreakVector _array_element)) 2e+02))))
    (Utilities|Array|AddUnique (Components|GetChildrenComponents (Variables|Default|GetSpawns) true) _returnvalue)))