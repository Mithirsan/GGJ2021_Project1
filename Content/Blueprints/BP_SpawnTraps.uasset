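; BP_SpawnTraps is a spawner that places a random number of randomly typed traps at predefined locations when play begins.
; It counts the ETrap enum entries and picks a count between MinimumTraps and the number of spawn locations.
; CompleteItemsToSpawn recursively fills ToSpawn with random trap types up to that count.
; SpawnItems shuffles the locations, spawns a BP_Trap at each chosen one and assigns its TrapType.
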(event Custom|SpawnItems
  ;[0 1 0] Comment
  (Utilities|Array|Shuffle (Variables|Default|GetSpawnsLocations))
  (for _index (range 0 (- (Utilities|Array|Length (Variables|Default|GetToSpawn)) 1))
    (bind _returnvalue (Game|SpawnActorfromClass "/Game/Blueprints/BP_Trap.BP_Trap_C" (Math|Transform|MakeTransform (Utilities|Array|Get(acopy) (Variables|Default|GetSpawnsLocations) _index) "0, 0, 0" "1,1,1") "AdjustIfPossibleButAlwaysSpawn" 0 0))
    ;;[1 1 1] Call function Set Mesh by type
    (Variables|/Game/Blueprints/BP_Trap.BP_Trap_C|SetTrapType _returnvalue (Utilities|Array|Get(acopy) (Variables|Default|GetToSpawn) _index))))

(event Custom|CompleteItemsToSpawn
  ;[0 1 0] Comment
  (if (< (Utilities|Array|Length (Variables|Default|GetToSpawn)) (Variables|Default|GetNumberOfItems))
    (Utilities|Array|Add (Variables|Default|GetToSpawn) (Utilities|Enum|ByteToEnumETrap (Math|Conversions|ToByte(Integer) (Math|Random|RandomIntegerinRange 0 (- (Variables|Default|GetNumberOfTrap) 1)))))
    (CallFunction|CompleteItemstoSpawn)))

(event EventBeginPlay
  ;[0 1 0] Comment
  (|ForEachETrap
    (:LoopBody
      (Math|Integer|IncrementInt (Variables|Default|GetNumberOfTrap)))
    (:then
      (Variables|Default|SetNumberOfItems (Math|Random|RandomIntegerinRange (Variables|Default|GetMinimumTraps) (Utilities|Array|Length (Variables|Default|GetSpawnsLocations))))
      (CallFunction|CompleteItemstoSpawn)
      (CallFunction|SpawnItems))))

(fn ConstructionScript)