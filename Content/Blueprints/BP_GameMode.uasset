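; Game mode that decides win or loss for a two-player game.
; BeginPlay creates the win and lose widgets and stores references to them.
; CheckWin shows the lose screen when both player characters have no health left.
; If either is alive and both report CanEscape, it shows the win screen, pausing the game in either outcome.
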(event Custom|CheckWin
  (if (or (> (Variables|/Game/Blueprints/BP_PlayerCharacter.BP_PlayerCharacter_C|GetHealth (.AsBP%20Player%20Character (Utilities|Casting|CastToBP_PlayerCharacter (Game|GetPlayerCharacter 0)))) 0.0) (> (Variables|/Game/Blueprints/BP_PlayerCharacter.BP_PlayerCharacter_C|GetHealth (.AsBP%20Player%20Character (Utilities|Casting|CastToBP_PlayerCharacter (Game|GetPlayerCharacter 1)))) 0.0))
    (if (and (Default|CanEscape (.AsBP%20Player%20Character (Utilities|Casting|CastToBP_PlayerCharacter (Game|GetPlayerCharacter 0)))) (Default|CanEscape (.AsBP%20Player%20Character (Utilities|Casting|CastToBP_PlayerCharacter (Game|GetPlayerCharacter 1)))))
      (Game|SetGamePaused true)
      (UserInterface|Viewport|AddtoViewport (Variables|Default|GetRefWinWidget) 0))
    (else
      (Game|SetGamePaused true)
      (UserInterface|Viewport|AddtoViewport (Variables|Default|GetRefLoseWidget) 0))))

(event EventBeginPlay
  (bind _returnvalue (Game|GetPlayerController 0))
  (bind _returnvalue_2 (UserInterface|CreateWidget "/Game/UI/W_Lose.W_Lose_C" _returnvalue))
  (Variables|Default|SetRefLoseWidget _returnvalue_2)
  (bind _returnvalue_3 (UserInterface|CreateWidget "/Game/UI/W_Win.W_Win_C" _returnvalue))
  (Variables|Default|SetRefWinWidget _returnvalue_3))

(fn ConstructionScript)