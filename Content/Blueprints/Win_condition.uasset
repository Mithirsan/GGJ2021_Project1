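; Win-condition Blueprint that decides whether a key passed to a door counts as a win.
; BeginPlay sets KeyLevel to true unconditionally.
; WinDoor compares its Key input to KeyLevel, sets DidWin on a match or DidLoose to false otherwise, then returns DidWin.
; Unconnected nodes hold checks for two player characters' picked-up keys, which never run.
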(event EventBeginPlay
  (Variables|Default|SetKey_Level true))

(event Collision|EventActorBeginOverlap
  (params (OtherActor :type Actor%20Object%20Reference)))

(event EventTick
  (params (DeltaSeconds :type Float%20%28single-precision%29)))

(fn ConstructionScript)

(fn WinDoor
  (params (Key :type Boolean))
  (if (Math|Boolean|Equal(Boolean) Key (Variables|Default|GetKey_Level))
    (LocalVariables|Setdid%20win true)
    (else
      (LocalVariables|Setdid%20loose false)))
  (return (LocalVariables|Getdid%20win)))