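; BP_Trap is a one-shot jaw trap that springs when any actor overlaps its box and damages the player.
; On overlap it plays the snap animation, removes the trigger box and activates a blood splash after a short delay.
; A timeline then ramps emissive on a dynamic metal material created in the construction script.
; When it finishes, a BP_PlayerCharacter victim takes damage by trap type and the trap destroys itself shortly after.
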(event OnComponentBeginOverlap(Box)
  (params (OverlappedComponent :type Primitive%20Component%20Object%20Reference) (OtherActor :type Actor%20Object%20Reference) (OtherComp :type Primitive%20Component%20Object%20Reference) (OtherBodyIndex :type Integer) (bFromSweep :type Boolean) (SweepResult :type Hit%20Result%20Structure%20%28by%20ref%29))
  (Components|Animation|PlayAnimation (Variables|Default|GetSkeletalMesh) "/Game/Geometry/PiegeALoup/SM_PiegeALoup_Anim.SM_PiegeALoup_Anim" false)
  (Components|DestroyComponent (Variables|Default|GetBox))
  (Utilities|FlowControl|Delay 0.2)
  (Components|Activation|SetActive (Variables|Default|GetBloodSplash) true false)
  (bind _fadeemissive (Timeline|FadeEmissive PlayFromStart)
    (:Update
      (Rendering|Material|SetScalarParameterValue (Variables|Default|GetDynaMat) "Emissive Scale" (Math|Float|Lerp 0.0 1e+02 _fadeemissive) :!class /Script/Engine.MaterialInstanceDynamic))
    (:Finished
      (bind _asbp_player_character (Utilities|Casting|CastToBP_PlayerCharacter OtherActor))
      (Default|TakeDamage _asbp_player_character (Variables|Default|GetTrapType))
      (Utilities|FlowControl|Delay 1.0)
      (Actor|DestroyActor))))

(fn ConstructionScript
  (bind _returnvalue (Rendering|Material|CreateDynamicMaterialInstance (Variables|Default|GetSkeletalMesh) 4 "/Game/Materials/MI_GenericMetal.MI_GenericMetal" "None" :!class /Script/Engine.PrimitiveComponent))
  (Variables|Default|SetDynaMat _returnvalue))