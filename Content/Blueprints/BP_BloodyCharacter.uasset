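; Player character Blueprint that moves with axis input and fires blood projectiles.
; Movement follows the control rotation, and BeginPlay calls Activate on Camera1 without reset.
; Fire spawns a Niagara blood burst and a BP_BloodProjectile at an offset from player 0, computed by crossing the mesh forward vector with world up.
; The burst takes the actor's rotation, while the projectile's transform carries only location.
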(event EventBeginPlay
  (Components|Activation|Activate (Variables|Default|GetCamera1) false))

(event Input|ActionEvents|InputActionFire
  (params (Key :type Key%20Structure :default "None"))
  (bind _returnvalue (Game|GetPlayerCharacter 0))
  (bind _returnvalue_2 (Transformation|GetActorLocation _returnvalue))
  (bind _mesh (Variables|/Script/Engine.Character|GetMesh _returnvalue))
  (bind _returnvalue_3 (Math|Vector|GetForwardVector _mesh))
  (bind _returnvalue_4 (Math|Vector|CrossProduct _returnvalue_3 "0,0.000000,1.000000"))
  (:Pressed
    (Niagara|SpawnSystematLocation "/Game/FX/NS_BloodBurst.NS_BloodBurst" (+ _returnvalue_2 (* _returnvalue_4 -2e+02)) (Transformation|GetActorRotation _returnvalue) "1.000000,1.000000,1.000000" false)
    (Game|SpawnActorfromClass "/Game/Blueprints/BP_BloodProjectile.BP_BloodProjectile_C" (Math|Conversions|ToTransform(Vector) (+ _returnvalue_2 (* _returnvalue_4 -2e+02))) "Undefined" 0 0)))

(event Input|AxisEvents|InputAxisMoveForward
  (params (AxisValue :type Float%20%28single-precision%29))
  (Pawn|Input|AddMovementInput (Math|Vector|GetForwardVector (Pawn|GetControlRotation :!class /Script/Engine.Pawn)) AxisValue false))

(event Input|AxisEvents|InputAxisMoveRight
  (params (AxisValue :type Float%20%28single-precision%29))
  (Pawn|Input|AddMovementInput (Math|Vector|GetRightVector (Pawn|GetControlRotation :!class /Script/Engine.Pawn)) AxisValue false))

(fn ConstructionScript)