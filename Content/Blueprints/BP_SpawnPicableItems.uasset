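; BP_SpawnPicableItems is a spawner that places a random number of pickable items at shuffled predefined locations on BeginPlay.
; It counts the EPickableItems entries, then recursively tops up ToSpawn with random types, leaving the last three enum entries out of the draw.
; Each spawned BP_PickableItem receives its type from that list.
; The construction script adds a box component at each spawn location.
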(event Custom|SpawnItems
  (Utilities|Array|Shuffle (Variables|Default|GetSpawnsLocations))
  (for _index (range 0 (- (Variables|Default|GetNumberOfItems) 1))
    (bind _returnvalue (Game|SpawnActorfromClass "/Game/Blueprints/BP_PickableItem.BP_PickableItem_C" (Math|Transform|MakeTransform (Utilities|Array|Get(acopy) (Variables|Default|GetSpawnsLocations) _index) "0, 0, 0" "1,1,1") "AdjustIfPossibleButAlwaysSpawn" 0 0))
    ;[1 1 1] Call function Set Mesh by type
    (Variables|/Game/Blueprints/BP_PickableItem.BP_PickableItem_C|SetItemType _returnvalue (Utilities|Array|Get(acopy) (Variables|Default|GetToSpawn) _index))))

(event Custom|CompleteItemsToSpawn
  (if (< (Utilities|Array|Length (Variables|Default|GetToSpawn)) (Variables|Default|GetNumberOfItems))
    (Utilities|Array|Add (Variables|Default|GetToSpawn) (Utilities|Enum|ByteToEnumEPickableItems (Math|Conversions|ToByte(Integer) (Math|Random|RandomInteger (- (Variables|Default|GetNimberOfPickableVariant) 3)))))
    (CallFunction|CompleteItemstoSpawn)))

(event EventBeginPlay
  (|ForEachEPickableItems
    (:LoopBody
      (Math|Integer|IncrementInt (Variables|Default|GetNimberOfPickableVariant)))
    (:then
      (Variables|Default|SetNumberOfItems (Math|Random|RandomIntegerinRange 6 (Utilities|Array|Length (Variables|Default|GetSpawnsLocations))))
      (CallFunction|CompleteItemstoSpawn)
      (CallFunction|SpawnItems))))

(fn ConstructionScript
  (for _array_element (Variables|Default|GetSpawnsLocations)
    (bind _returnvalue (AddComponent|AddBoxComponent true (Math|Transform|MakeTransform _array_element)))
    (Utilities|Array|AddUnique (Components|GetChildrenComponents (Variables|Default|GetROOT) true) _returnvalue)))