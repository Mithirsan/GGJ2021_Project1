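; Player character that uses its own health as ammunition while collecting items to escape.
; Firing spawns a blood burst and projectile, costs health and starts timed bleeding, gated by a cooldown.
; A self-recalling one-second loop drains health while bleeding and asks BP_GameMode to check the win state at zero health.
; PickItem handles healing and two keys for CanEscape, while TakeDamage applies identical damage for every trap type, with per-type actions unfinished.
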(event Custom|PlayerIsBleeding
  ;[1 1 1] Comment
  (if (Variables|Default|GetIsBleeding?)
    (Components|Activation|SetActive (Variables|Default|GetBloodDrops) true true)
    (bind _output_get (Variables|Default|SetHealth (- (Variables|Default|GetHealth) 5.0)))
    (else
      (Components|Activation|SetActive (Variables|Default|GetBloodDrops) false true)))
  (if (<= _output_get 0.0)
    (Default|CheckWin (.AsBP%20Game%20Mode (Utilities|Casting|CastToBP_GameMode (Game|GetGameMode))))
    (else
      (Utilities|FlowControl|Delay 1.0)
      (CallFunction|PlayerIsBleeding))))

(event Custom|BleedingDuration
  (params (Duration :type Float%20%28single-precision%29))
  ;[1 1 1] Comment
  (Variables|Default|SetIsBleeding? true)
  (Utilities|FlowControl|Delay Duration)
  (Variables|Default|SetIsBleeding? false))

(event EventBeginPlay
  (CallFunction|PlayerIsBleeding)
  (Variables|Default|SetHealth (Variables|/Game/Blueprints/BP_GameMode.BP_GameMode_C|GetPlayerMaxHealth (.AsBP%20Game%20Mode (Utilities|Casting|CastToBP_GameMode (Game|GetGameMode))))))

(event Input|ActionEvents|InputActionFire
  (params (Key :type Key%20Structure :default "None"))
  (bind _returnvalue (Transformation|GetActorLocation))
  (bind _returnvalue_2 (Transformation|GetActorRotation))
  (bind _mesh (Variables|Character|GetMesh))
  (bind (_roll _pitch _yaw) (Math|Rotator|BreakRotator _returnvalue_2))
  (bind _returnvalue_3 (Math|Vector|GetForwardVector _mesh))
  (bind _returnvalue_4 (Math|Vector|CrossProduct _returnvalue_3 "0, 0,1.000000"))
  (bind _returnvalue_5 (* _returnvalue_4 -2e+02))
  (bind _returnvalue_6 (+ _returnvalue _returnvalue_5))
  ;[0 1 0] Spawn Projectile at location, lose hp
  (:Pressed
    (if (not (Variables|Default|GetIsOnCoolDown?))
      (Variables|Default|SetIsOnCoolDown? true)
      (Niagara|SpawnSystematLocation "/Game/FX/NS_BloodBurst.NS_BloodBurst" _returnvalue_6 (Transformation|GetActorRotation) "1.000000,1.000000,1.000000" false)
      (Game|SpawnActorfromClass "/Game/Blueprints/BP_BloodProjectile.BP_BloodProjectile_C" (Math|Transform|MakeTransform _returnvalue_6 (Math|Rotator|MakeRotator 0.0 _pitch _yaw)) "Undefined" 0 0)
      (Variables|Default|SetHealth (- (Variables|Default|GetHealth) 5.0))
      (CallFunction|BleedingDuration 5.0)
      (Utilities|FlowControl|Delay 2.0)
      (Variables|Default|SetIsOnCoolDown? false))))

(event Input|AxisEvents|InputAxisMoveForward
  (params (AxisValue :type Float%20%28single-precision%29))
  ;[0 1 0] 2 axis Movement
  (Pawn|Input|AddMovementInput (Math|Vector|GetForwardVector (Pawn|GetControlRotation :!class /Script/Engine.Pawn)) AxisValue false))

(event Input|AxisEvents|InputAxisMoveRight
  (params (AxisValue :type Float%20%28single-precision%29))
  ;[0 1 0] 2 axis Movement
  (Pawn|Input|AddMovementInput (Math|Vector|GetRightVector (Pawn|GetControlRotation :!class /Script/Engine.Pawn)) AxisValue false))

(fn ConstructionScript)

(fn PickItem
  (params (Item :type EPickableItems%20Enum :default "EPickableItems_MAX"))
  (LocalVariables|SetPicked false)
  (switch Utilities|FlowControl|Switch|SwitchonEPickableItems Item
    (:NewEnumerator1
      ;[1 1 1] TODO :: Define actions for each
      (Variables|Default|SetHealth (+ (Variables|Default|GetHealth) 15.0))
      (LocalVariables|SetPicked true))
    (:NewEnumerator7
      ;[0 1 0] Pick First Key if not already Picked
      (if (Variables|Default|GetAsPickedKey1?)
        _
        (else
          (Variables|Default|SetAsPickedKey1? true)
          (LocalVariables|SetPicked true))))
    (:NewEnumerator8
      ;[0 1 0] Pick Second Key if not already Picked
      (if (Variables|Default|GetAsPickedKey2?)
        _
        (else
          (Variables|Default|SetAsPickedKey2? true)
          (LocalVariables|SetPicked true)))))
  (return (LocalVariables|GetPicked)))

(fn TakeDamage
  (params (Trap%20Type :type ETrap%20Enum :default "NewEnumerator0"))
  (switch Utilities|FlowControl|Switch|SwitchonETrap Trap%20Type
    (:NewEnumerator0
      _)
    (:NewEnumerator1
      _)
    (:NewEnumerator2
      _)
    (:NewEnumerator3
      _)
    (:NewEnumerator4
      _)
    (:NewEnumerator5
      _)
    (:NewEnumerator6
      _))
  ;[1 1 1] TODO :: Define actions for each
  (Variables|Default|SetHealth (+ (Variables|Default|GetHealth) -15.0))
  (Default|CheckWin (.AsBP%20Game%20Mode (Utilities|Casting|CastToBP_GameMode (Game|GetGameMode)))))

(fn CanEscape
  (return (Math|Boolean|ANDBoolean (Variables|Default|GetAsPickedKey1?) (Variables|Default|GetAsPickedKey2?) (Variables|Default|GetIsWaitingToGoOut?))))