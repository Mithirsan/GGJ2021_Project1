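; BP_BloodProjectile is a projectile actor that leaves a blood decal where it hits.
; SetVolicityByPlayerId sets its ProjectileMovement velocity along the capsule forward vector of the player character with the given index, at a fixed speed.
; When its Box begins any overlap, it spawns BP_BloodDecal at its location, prints a debug message and destroys itself.
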(event OnComponentBeginOverlap(Box)
  (params (OverlappedComponent :type Primitive%20Component%20Object%20Reference) (OtherActor :type Actor%20Object%20Reference) (OtherComp :type Primitive%20Component%20Object%20Reference) (OtherBodyIndex :type Integer) (bFromSweep :type Boolean) (SweepResult :type Hit%20Result%20Structure%20%28by%20ref%29))
  (Game|SpawnActorfromClass "/Game/FX/Blueprints/BP_bloodDecal.BP_BloodDecal_C" (Math|Conversions|ToTransform(Vector) (Transformation|GetActorLocation)) "Undefined" 0 0)
  (Development|PrintString "hit")
  (Actor|DestroyActor))

(fn ConstructionScript)

(fn SetVolicitybyPlayerId
  (params (Id :type Integer))
  (Variables|/Script/Engine.MovementComponent|SetVelocity (Variables|Default|GetProjectileMovement) (* (Math|Vector|GetForwardVector (Variables|/Script/Engine.Character|GetCapsuleComponent (Game|GetPlayerCharacter Id))) 1e+03))
  (return))