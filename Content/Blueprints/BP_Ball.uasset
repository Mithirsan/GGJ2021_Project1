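; BP_Ball is a thrown projectile, apparently a blood glob, that leaves a decal where it lands.
; On BeginPlay it adds a projectile movement component at runtime, launching it forward at a speed set by BloodThrowingDistance with rotation following velocity.
; When its collision overlaps an actor tagged "Blood", it prints a debug string, spawns BP_DecalTest at its location with zero rotation, then destroys itself.
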(event OnComponentBeginOverlap(collision)
  (params (OverlappedComponent :type Primitive%20Component%20Object%20Reference) (OtherActor :type Actor%20Object%20Reference) (OtherComp :type Primitive%20Component%20Object%20Reference) (OtherBodyIndex :type Integer) (bFromSweep :type Boolean) (SweepResult :type Hit%20Result%20Structure%20%28by%20ref%29))
  (if (Actor|ActorHasTag OtherActor "Blood")
    (Development|PrintString "Hello")
    (Game|SpawnActorfromClass "/Game/Blueprints/BP_DecalTest.BP_DecalTest_C" (Math|Transform|MakeTransform (Transformation|GetActorLocation)) "AdjustIfPossibleButAlwaysSpawn" 0 0)
    (Actor|DestroyActor)))

(event EventBeginPlay
  (bind _returnvalue (AddComponent|AddProjectileMovementComponent))
  (Variables|/Script/Engine.MovementComponent|SetVelocity _returnvalue (* (Transformation|GetActorForwardVector) (Variables|Default|GetBloodThrowingDistance)))
  (Variables|/Script/Engine.ProjectileMovementComponent|SetbRotationFollowsVelocity _returnvalue true))

(fn ConstructionScript)