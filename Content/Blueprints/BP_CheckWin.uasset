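; BP_CheckWin is an exit trigger that marks a player character as waiting to go out and asks the game mode to check for a win.
; When a BP_PlayerCharacter enters Trigger1, it sets IsWaitingToGoOut, lights PointLight1 green and calls CheckWin on BP_GameMode.
; When that character leaves, it clears the flag and turns the light off.
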(event OnComponentBeginOverlap(Trigger1)
  (params (OverlappedComponent :type Primitive%20Component%20Object%20Reference) (OtherActor :type Actor%20Object%20Reference) (OtherComp :type Primitive%20Component%20Object%20Reference) (OtherBodyIndex :type Integer) (bFromSweep :type Boolean) (SweepResult :type Hit%20Result%20Structure%20%28by%20ref%29))
  ;[1 1 1] Comment
  (bind _asbp_player_character (Utilities|Casting|CastToBP_PlayerCharacter OtherActor))
  (Variables|/Game/Blueprints/BP_PlayerCharacter.BP_PlayerCharacter_C|SetIsWaitingToGoOut? _asbp_player_character true)
  (Rendering|Components|Light|SetIntensity (Variables|Default|GetPointLight1) 5e+01)
  (if true
    (Rendering|Components|Light|SetLightColor (Variables|Default|GetPointLight1) "(R=0.000000,G=1.000000,B=0.000000,A=1.000000)" true)
    (Default|CheckWin (.AsBP%20Game%20Mode (Utilities|Casting|CastToBP_GameMode (Game|GetGameMode))))))

(event OnComponentEndOverlap(Trigger1)
  (params (OverlappedComponent :type Primitive%20Component%20Object%20Reference) (OtherActor :type Actor%20Object%20Reference) (OtherComp :type Primitive%20Component%20Object%20Reference) (OtherBodyIndex :type Integer))
  (bind _pointlight1 (Variables|Default|GetPointLight1))
  ;[1 1 1] Comment
  (bind _asbp_player_character (Utilities|Casting|CastToBP_PlayerCharacter OtherActor))
  (Variables|/Game/Blueprints/BP_PlayerCharacter.BP_PlayerCharacter_C|SetIsWaitingToGoOut? _asbp_player_character false)
  (Rendering|Components|Light|SetLightColor _pointlight1 "(R=0.000000,G=0.000000,B=0.000000,A=1.000000)" true)
  (Rendering|Components|Light|SetIntensity _pointlight1 0.0))

(fn ConstructionScript)