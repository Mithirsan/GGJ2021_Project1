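; Projectile Blueprint that leaves a glowing blood decal when its Box begins overlapping something.
; It spawns BP_bloodDecal at the Box's location and gives the decal a dynamic material instance.
; The FadeLight timeline then drives the decal actor's spotlight intensity, with debug prints along the way.
; Random splash frame, emissive scaling and FadeOut logic are present but disconnected, so they never run.
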(event OnComponentBeginOverlap(Box)
  (params (OverlappedComponent :type Primitive%20Component%20Object%20Reference) (OtherActor :type Actor%20Object%20Reference) (OtherComp :type Primitive%20Component%20Object%20Reference) (OtherBodyIndex :type Integer) (bFromSweep :type Boolean) (SweepResult :type Hit%20Result%20Structure%20%28by%20ref%29))
  (Development|PrintString "collide")
  (bind _returnvalue (Game|SpawnActorfromClass "/Game/FX/Blueprints/BP_bloodDecal.BP_bloodDecal_C" (Math|Conversions|ToTransform(Vector) (Transformation|GetWorldLocation OverlappedComponent)) "Undefined" 0 0))
  (bind _output_get (Variables|Default|SetBPDecal _returnvalue))
  (bind _returnvalue_2 (Rendering|Material|CreateDynamicMaterialInstance (Variables|/Game/FX/Blueprints/BP_bloodDecal.BP_bloodDecal_C|GetDecal _output_get) :!class /Script/Engine.DecalComponent))
  (bind _output_get_2 (Variables|Default|SetDynaDecalMat _returnvalue_2))
  (Rendering|Components|Decal|SetDecalMaterial (Variables|/Game/FX/Blueprints/BP_bloodDecal.BP_bloodDecal_C|GetDecal (Variables|Default|GetBPDecal)) _output_get_2)
  (bind _fade (Timeline|FadeLight PlayFromStart)
    (:Update
      (Development|PrintString (Utilities|String|ToString(Float) (* _fade 1e+03)))
      (Rendering|Components|Light|SetIntensity (Variables|/Game/FX/Blueprints/BP_bloodDecal.BP_bloodDecal_C|GetSpotLight (Variables|Default|GetBPDecal)) (* _fade 1e+06)))))

(fn ConstructionScript)