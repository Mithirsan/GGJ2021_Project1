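; BP_bloodDecal is a short-lived blood decal actor with a glowing material and spot light that destroys itself after fading out.
; On BeginPlay it creates a dynamic decal material, then a timeline ramps the light while setting emissive straight to full intensity, despite the fade-in comment.
; After a brief delay, a second timeline lerps both emissive and light intensity for the fade-out, with debug prints throughout.
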(event EventBeginPlay
  (bind _returnvalue (Rendering|Material|CreateDynamicMaterialInstance (Variables|Default|GetDecal) :!class /Script/Engine.DecalComponent))
  (bind _output_get (Variables|Default|SetDynaDecalMat _returnvalue))
  (Rendering|Components|Decal|SetDecalMaterial (Variables|Default|GetDecal) _output_get)
  (bind _newtrack_0 (Timeline|Timeline_0 Play)
    (:Update
      (Development|PrintString (Utilities|String|ToString(Float) _newtrack_0) false)
      ;[1 1 1] Fade in emissive
      (Rendering|Material|SetScalarParameterValue (Variables|Default|GetDynaDecalMat) "Emissive scale" (Variables|Default|GetEmissiveIntensity) :!class /Script/Engine.MaterialInstanceDynamic)
      ;[1 1 1] Fade in light
      (Rendering|Components|Light|SetIntensity (Variables|Default|GetSpotLight) (* _newtrack_0 (Variables|Default|GetLightIntensity))))
    (:Finished
      ;[1 1 1] Delayt before fadeout
      (Development|PrintString "Finished")
      (Utilities|FlowControl|Delay 0.2)
      (bind _fade_out (Timeline|Timeline_1 Play)
        (:Update
          (Development|PrintString (Utilities|String|ToString(Float) _fade_out) false)
          (Rendering|Material|SetScalarParameterValue (Variables|Default|GetDynaDecalMat) "Emissive scale" (Math|Float|Lerp 0.0 (Variables|Default|GetEmissiveIntensity) _fade_out) :!class /Script/Engine.MaterialInstanceDynamic)
          (Rendering|Components|Light|SetIntensity (Variables|Default|GetSpotLight) (Math|Float|Lerp 0.0 (Variables|Default|GetLightIntensity) _fade_out)))
        (:Finished
          (Development|PrintString "fINISHED FADE OUT")
          (Actor|DestroyActor))))))

(fn ConstructionScript)