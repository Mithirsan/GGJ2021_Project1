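; Modular wall door Blueprint that swings open automatically when an actor overlaps its box trigger and closes when the overlap ends.
; The overlapping actor's position, converted into the door's local space, picks a positive or negative 90-degree yaw by side.
; OpenSwing and CloseSwing timelines lerp DoorPivot's relative rotation from its current value, each stopping the other, with a sound played at each change.
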(event OnComponentBeginOverlap(Box)
  (params (OverlappedComponent :type Primitive%20Component%20Object%20Reference) (OtherActor :type Actor%20Object%20Reference) (OtherComp :type Primitive%20Component%20Object%20Reference) (OtherBodyIndex :type Integer) (bFromSweep :type Boolean) (SweepResult :type Hit%20Result%20Structure%20%28by%20ref%29))
  (bind _returnvalue (Transformation|GetActorLocation))
  (bind _door_pivot (Variables|Default|Getdoor_pivot))
  ;[1 1 1] Comment
  ;;[1 1 1] Comment
  (Audio|PlaySoundatLocation 0 _returnvalue "0, 0, 0" 1.0 1.0 0.0 0 0 0)
  (Audio|Components|Audio|Stop (Variables|Default|GetCloseSwing))
  (Variables|Default|SetOpenDirection (< (.Y (Math|Vector|BreakVector (Math|Vector|UnrotateVector (- _returnvalue (Transformation|GetActorLocation OtherActor)) (Transformation|GetActorRotation)))) 0.0))
  (bind _open (Timeline|OpenSwing PlayFromStart)
    (:Update
      (Transformation|SetRelativeRotation _door_pivot (Math|Rotator|Lerp(Rotator) (Variables|/Script/Engine.SceneComponent|GetRelativeRotation _door_pivot) (Math|Rotator|MakeRotator 0.0 0.0 (Math|Float|SelectFloat 9e+01 -9e+01 (Variables|Default|GetOpenDirection))) _open true) false false))))

(event OnComponentEndOverlap(Box)
  (params (OverlappedComponent :type Primitive%20Component%20Object%20Reference) (OtherActor :type Actor%20Object%20Reference) (OtherComp :type Primitive%20Component%20Object%20Reference) (OtherBodyIndex :type Integer))
  (bind _door_pivot (Variables|Default|Getdoor_pivot))
  ;[1 1 1] Comment
  ;;[1 1 1] Comment
  (Audio|PlaySoundatLocation 0 (Transformation|GetActorLocation) "0, 0, 0" 1.0 1.0 0.0 0 0 0)
  (Audio|Components|Audio|Stop (Variables|Default|GetOpenSwing))
  (bind _close (Timeline|CloseSwing PlayFromStart)
    (:Update
      (Transformation|SetRelativeRotation _door_pivot (Math|Rotator|Lerp(Rotator) (Variables|/Script/Engine.SceneComponent|GetRelativeRotation _door_pivot) "0, 0, 0" _close true) false false))))

(fn ConstructionScript)